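; BP_Charger is the Charger enemy Blueprint, which mirrors part of its AI state onto itself.
; Every Tick it casts its controller to BP_Charger_AIController and copies the SeenPlayer, IsCharging and CanCharge Blackboard bools into matching variables.
; It holds no charge logic of its own, and its BeginPlay, overlap event and construction script are empty.
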(event EventBeginPlay)

(event Collision|EventActorBeginOverlap
  (params (OtherActor :type Actor%20Object%20Reference)))

(event EventTick
  (params (DeltaSeconds :type Float%20%28single-precision%29))
  (bind _asbp_charger_aicontroller (Utilities|Casting|CastToBP_Charger_AIController (Pawn|GetController)))
  (Variables|Default|SetSeenPlayer (ScalableFloat|GetValueasBool (Variables|/Script/AIModule.AIController|GetBlackboard _asbp_charger_aicontroller) (Utilities|String|StringToName "SeenPlayer")))
  (Variables|Default|SetIsCharging (ScalableFloat|GetValueasBool (Variables|/Script/AIModule.AIController|GetBlackboard _asbp_charger_aicontroller) (Utilities|String|StringToName "IsCharging")))
  (Variables|Default|SetCanCharge (ScalableFloat|GetValueasBool (Variables|/Script/AIModule.AIController|GetBlackboard _asbp_charger_aicontroller) (Utilities|String|StringToName "CanCharge"))))

(fn ConstructionScript)